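; Modular anime character Blueprint that builds a randomized male or female look in its construction script.
; It flips a coin for gender, picks the matching fixed head, then random torso, bottom and hair meshes from per-gender arrays.
; AnimeShading sets up the parts, FaceAnimation receives the head, and fixed per-gender skin and face materials are applied.
; Getters expose the face animation component and look point.
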(fn ConstructionScript
  (bind _mesh (Variables|Character|GetMesh))
  (bind _hair (Variables|Default|GetHair))
  (Variables|Default|SetIsFem (Math|Random|RandomBool))
  (Variables|Appearance|SetHeadMesh (select (Variables|Default|GetIsFem) "/Game/AnimeCharacters/Blueprints/Characters/Female_Average/Head/Starter/skl_AnimeF_Head_1.skl_AnimeF_Head_1" "/Game/AnimeCharacters/Blueprints/Characters/Male_Average/Head/Starter/skl_AnimeM_Head_0.skl_AnimeM_Head_0"))
  (Variables|Appearance|SetTorsoMesh (select (Variables|Default|GetIsFem) (.OutItem (Utilities|Array|Random (Variables|Default|GetFemaleTorso))) (.OutItem (Utilities|Array|Random (Variables|Default|GetMaleTorso)))))
  (Variables|Appearance|SetBottomMesh (select (Variables|Default|GetIsFem) (.OutItem (Utilities|Array|Random (Variables|Default|GetFemaleBottom))) (.OutItem (Utilities|Array|Random (Variables|Default|GetMaleBottom)))))
  (Variables|Appearance|SetHairMesh (select (Variables|Default|GetIsFem) (.OutItem (Utilities|Array|Random (Variables|Default|GetFemaleHair))) (.OutItem (Utilities|Array|Random (Variables|Default|GetMaleHair)))))
  (Default|SetupCharacter (Variables|Default|GetAnimeShading) _mesh _hair (Utilities|Array|MakeArray _mesh (Variables|Default|GetTop) (Variables|Default|GetBottom) _hair) (Utilities|Array|MakeArray (Variables|Appearance|GetHeadMesh) (Variables|Appearance|GetTorsoMesh) (Variables|Appearance|GetBottomMesh) (Variables|Appearance|GetHairMesh)))
  (Default|SetHeadComponent (Variables|Default|GetFaceAnimation) (Variables|Character|GetMesh))
  (if (Variables|Default|GetIsFem)
    (Rendering|Material|SetMaterial (Variables|Default|GetBottom) 0 (Utilities|Array|Get(acopy) (Variables|Default|GetFemaleSkinMat) 1))
    (Rendering|Material|SetMaterial (Variables|Character|GetMesh) 0 (Utilities|Array|Get(acopy) (Variables|Default|GetFemaleFaceMat) 1))
    (else
      (Rendering|Material|SetMaterial (Variables|Default|GetBottom) 0 (Utilities|Array|Get(acopy) (Variables|Default|GetMaleSkinMat) 1))
      (Rendering|Material|SetMaterial (Variables|Character|GetMesh) 2 (Utilities|Array|Get(acopy) (Variables|Default|GetMaleFaceMat) 1)))))

(fn GetAnimeAnimationComponent
  (return (Variables|Default|GetFaceAnimation)))

(fn GetAnimLookPoint
  (return (Variables|Default|GetLookPoint)))