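; BP_Item is a world item that acts as either a food/trash station or a three-item order showing icon bubbles.
; With Bubble and Icon set it becomes a granter, giving that item on box overlap or removing one if Trash.
; Otherwise it shows random icons; a matching character delivers, triggers FriendManager's MoveChars and destroys it.
; SameItems matches order-independently by requiring even combined Burger, Fries and Soda counts, a parity check rather than strict equality.
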(event OnComponentBeginOverlap(Box)
  (params (OverlappedComponent :type Primitive%20Component%20Object%20Reference) (OtherActor :type Actor%20Object%20Reference) (OtherComp :type Primitive%20Component%20Object%20Reference) (OtherBodyIndex :type Integer) (bFromSweep :type Boolean) (SweepResult :type Hit%20Result%20Structure%20%28by%20ref%29))
  (bind _icon (Variables|Default|GetIcon))
  (bind _asbp_top_down_character (Utilities|Casting|CastToBP_TopDownCharacter OtherActor))
  (if (Variables|Default|GetIsGranter)
    (if (== _icon "/Game/UI/Textures/Trash.Trash")
      (Default|RemoveItem _asbp_top_down_character)
      (else
        (Default|ReceiveItem _asbp_top_down_character _icon)))
    (else
      (bind _equal (CallFunction|SameItems (Default|GetIconArray _asbp_top_down_character) (Utilities|Array|MakeArray (Variables|/Game/UI/W_Icon.W_Icon_C|GetIcon (Variables|Default|GetIcon1)) (Variables|/Game/UI/W_Icon.W_Icon_C|GetIcon (Variables|Default|GetIcon2)) (Variables|/Game/UI/W_Icon.W_Icon_C|GetIcon (Variables|Default|GetIcon3)))))
      (if _equal
        (Default|DeliverItems _asbp_top_down_character)
        (Default|MoveChars (Variables|Default|GetFriendManager))
        (Actor|DestroyActor)))))

(event EventBeginPlay
  (bind _returnvalue (Actor|GetActorOfClass "/Game/Blueprints/BP_FriendingManager.BP_FriendingManager_C"))
  (Variables|Default|SetFriendManager _returnvalue)
  (bind _asw_icon (Utilities|Casting|CastToW_Icon (UserInterface|GetWidget (Variables|Default|GetWidget))))
  (bind _output_get (Variables|Default|SetIcon1 _asw_icon))
  (bind _bubble (Variables|Default|GetBubble)
    (:then
      (bind _icon (Variables|Default|GetIcon)
        (:then
          (Default|ShowWidget _output_get _bubble _icon)
          (Components|DestroyComponent (Variables|Default|GetWidget1))
          (Variables|Default|SetIsGranter true))
        (:else
          (Default|ShowWidget _output_get "/Game/UI/Textures/speech-bubble-icon-2048x1957-nda.speech-bubble-icon-2048x1957-nda" (.OutItem (Utilities|Array|Random (Variables|Default|GetList))) :!label _label)
          (bind _asw_icon_2 (Utilities|Casting|CastToW_Icon (UserInterface|GetWidget (Variables|Default|GetWidget1))))
          (bind _output_get_2 (Variables|Default|SetIcon2 _asw_icon_2))
          (Default|ShowWidget _output_get_2 "/Game/UI/Textures/speech-bubble-icon-2048x1957-nda.speech-bubble-icon-2048x1957-nda" (.OutItem (Utilities|Array|Random (Variables|Default|GetList))))
          (bind _asw_icon_3 (Utilities|Casting|CastToW_Icon (UserInterface|GetWidget (Variables|Default|GetWidget2))))
          (bind _output_get_3 (Variables|Default|SetIcon3 _asw_icon_3))
          (Default|ShowWidget _output_get_3 "/Game/UI/Textures/speech-bubble-icon-2048x1957-nda.speech-bubble-icon-2048x1957-nda" (.OutItem (Utilities|Array|Random (Variables|Default|GetList)))))))
    (:else
      (goto _label))))

(event Collision|EventActorBeginOverlap
  (params (OtherActor :type Actor%20Object%20Reference)))

(fn ConstructionScript)

(fn SameItems
  (params (First%20Items :type Array%20of%20Texture%202D%20Object%20References) (Second%20Items :type Array%20of%20Texture%202D%20Object%20References))
  (bind _count (LocalVariables|GetCount))
  (for _array_element First%20Items
    (Utilities|Map|Add (LocalVariables|GetCount) _array_element (Math|Integer|SelectInt (+ (.Value (Utilities|Map|Find (LocalVariables|GetCount) _array_element)) 1) 1 (.ReturnValue (Utilities|Map|Find (LocalVariables|GetCount) _array_element)))))
  (for _array_element_2 Second%20Items
    (Utilities|Map|Add (LocalVariables|GetCount) _array_element_2 (Math|Integer|SelectInt (+ (.Value (Utilities|Map|Find (LocalVariables|GetCount) _array_element_2)) 1) 1 (.ReturnValue (Utilities|Map|Find (LocalVariables|GetCount) _array_element_2)))))
  (return (Math|Boolean|ANDBoolean (== (Math|Integer|%(Integer) (.Value (Utilities|Map|Find _count "/Game/UI/Textures/Burger.Burger")) 2) 0) (== (Math|Integer|%(Integer) (.Value (Utilities|Map|Find _count "/Game/UI/Textures/Fries.Fries")) 2) 0) (== (Math|Integer|%(Integer) (.Value (Utilities|Map|Find _count "/Game/UI/Textures/Soda.Soda")) 2) 0))))