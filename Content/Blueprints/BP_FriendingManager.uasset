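; Manager for the friending sequence that shuffles a group of AI friend characters around fixed spots and signals game completion.
; BeginPlay records each friend's transform, using DelilahPoint in place of Delilah, who walks there through a separate entrance event.
; Each MoveChars call increments an offset and sends every friend via BP_MNAIController to the wrapped next spot and its rotation.
; Once the offset reaches four, it calls game complete after a short delay.
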(event Custom|MoveChars
  (bind _friends (Variables|Default|GetFriends))
  (bind _returnvalue (Utilities|Array|Length _friends))
  (Math|Integer|IncrementInt (Variables|Default|GetOffset)
    (:%20%20
      (for (_array_element _array_index) _friends
        (bind _asbp_mnaicontroller (Utilities|Casting|CastToBP_MNAIController (AI|GetAIController _array_element)))
        (AI|ClearFocus _asbp_mnaicontroller)
        (Variables|/Game/Blueprints/BP_MNAIController.BP_MNAIController_C|SetDesiredRotation _asbp_mnaicontroller (.rotation (Utilities|Array|Get(acopy) (Variables|Default|GetLocations) (Math|Integer|SelectInt (- (+ _array_index (Variables|Default|GetOffset)) _returnvalue) (+ _array_index (Variables|Default|GetOffset)) (>= (+ _array_index (Variables|Default|GetOffset)) _returnvalue)))))
        (AI|Navigation|MovetoLocation _asbp_mnaicontroller (.location (Utilities|Array|Get(acopy) (Variables|Default|GetLocations) (Math|Integer|SelectInt (- (+ _array_index (Variables|Default|GetOffset)) _returnvalue) (+ _array_index (Variables|Default|GetOffset)) (>= (+ _array_index (Variables|Default|GetOffset)) _returnvalue)))) 1.0 false true true true 0))
      (if (>= (Variables|Default|GetOffset) 4)
        (Utilities|FlowControl|Delay 1.0)
        (Default|CallGameComplete)))))

(event Custom|DelilahEntrance
  (bind _delilahpoint (Variables|Default|GetDelilahPoint))
  (bind _returnvalue (Transformation|GetActorTransform _delilahpoint))
  (bind _asbp_mnaicontroller (Utilities|Casting|CastToBP_MNAIController (AI|GetAIController (Variables|Default|GetDelilah))))
  (AI|ClearFocus _asbp_mnaicontroller)
  (Variables|/Game/Blueprints/BP_MNAIController.BP_MNAIController_C|SetDesiredRotation _asbp_mnaicontroller (.rotation _returnvalue))
  (AI|Navigation|MovetoLocation _asbp_mnaicontroller (.location _returnvalue) 1.0 false true true true 0))

(event EventBeginPlay
  (for _array_element (Variables|Default|GetFriends)
    (Utilities|Array|Add (Variables|Default|GetLocations) (Transformation|GetActorTransform (select (== _array_element (Variables|Default|GetDelilah)) (Variables|Default|GetDelilahPoint) _array_element)))))

(fn ConstructionScript)